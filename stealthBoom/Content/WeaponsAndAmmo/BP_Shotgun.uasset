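; Shotgun weapon Blueprint that extends a parent weapon's Shoot and laser pointer functions.
; Shoot plays the firing animation and sound, then fires multiple randomly spread line traces from the Ammo socket to mimic pellets.
; Each hit applies damage, spawning a blood decal actor on guard enemies or an attached, temporary bullet-hole decal on anything else.
; The laser pointer function toggles the shotgun laser's visibility and prints its state.
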(fn `LaserPointerXD`
  (bind _shotgunlaser (`self.ShotGunLaser`))
  (`parent.LaserPointerXD`)
  (if (`self.laser visible`)
    (`SceneComponent.SetVisibility` _shotgunlaser false false)
    (`KismetSystemLibrary.PrintString` "Toggle off")
    (set `self.laser visible` false)
    (else
      (`SceneComponent.SetVisibility` _shotgunlaser true false)
      (`KismetSystemLibrary.PrintString` "Toggle on")
      (set `self.laser visible` true))))

(fn `Shoot`
  (bind _weaponskeletalmesh (`self.WeaponSkeletalmesh`))
  (bind _spread_0 (`self.Spread_0`))
  (bind _spread_0_2 (`self.Spread_0`))
  (bind _spread_0_3 (`self.Spread_0`))
  (bind (_returnvalue_location _returnvalue_rotation) (`KismetMathLibrary.BreakTransform` (`SceneComponent.GetSocketTransform` _weaponskeletalmesh "Ammo" "RTS_World")))
  (`parent.Shoot`)
  (`SkeletalMeshComponent.PlayAnimation` _weaponskeletalmesh "/Game/WeaponsAndAmmo/SM_Shotgun_01_Skel_Sequence.SM_Shotgun_01_Skel_Sequence" false)
  (`GameplayStatics.PlaySoundAtLocation` "/Game/FirstPerson/Blueprints/GunSounds/Shotgun.Shotgun" _returnvalue_location (struct) 1.0 1.0 0.0 null null null null)
  ;[1 1 1] multiple linetracer to mimic shot gun pellets
  (for _ (range 11)
    (bind (_outhit _returnvalue) (`KismetSystemLibrary.LineTraceSingle` :`Start` _returnvalue_location :`End` (+ (`SceneComponent.K2_GetComponentLocation` _weaponskeletalmesh) (* (`KismetMathLibrary.GetForwardVector` _returnvalue_rotation) 10000.0) (`KismetMathLibrary.MakeVector` (`KismetMathLibrary.RandomFloatInRange` (* _spread_0_2 -1.0) _spread_0_2) (`KismetMathLibrary.RandomFloatInRange` (* _spread_0_3 -1.0) _spread_0_3) (`KismetMathLibrary.RandomFloatInRange` (* _spread_0 -1.0) _spread_0))) :`TraceChannel` "TraceTypeQuery3" :`DrawDebugType` "ForOneFrame" :`TraceColor` (struct :`R` 0.55 :`A` 1.0)))
    (if _returnvalue
      (bind (_bblockinghit _binitialoverlap _time _distance _location _impactpoint _normal _impactnormal _physmat _hitactor _hitcomponent) (`GameplayStatics.BreakHitResult` _outhit))
      (`GameplayStatics.ApplyDamage` _hitactor 12.0)
      (cast `/Game/Enemies/AI/BP_Enemy_Base_Guard` _hitactor
        (:`then`
          ;[0.487 0.001268 0.004079] Bloodsplatter
          (`|SpawnActorFromClass` "/Game/Megascans/Decals/blooddecal.blooddecal_C" (`KismetMathLibrary.MakeTransform` _location (`KismetMathLibrary.Conv_VectorToRotator` _impactnormal)) "Undefined" "MultiplyWithRoot" null null))
        (:`CastFailed`
          ;[0.3333 0.3333 0.3333] BULLET HOLE decal when hit looks wierd on ground what can i do :-D
          (`GameplayStatics.SpawnDecalAttached` "/Game/WeaponsAndAmmo/BulletHoleMaterial.BulletHoleMaterial" (10.0 10.0 10.0) _hitcomponent "None" _location (struct) "KeepWorldPosition" 10.0))))))

(fn `UserConstructionScript`
  (`parent.UserConstructionScript`))