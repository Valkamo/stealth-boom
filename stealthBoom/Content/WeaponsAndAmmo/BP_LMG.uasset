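; LMG weapon Blueprint that extends a parent weapon's shoot, laser pointer and reload functions.
; Shoot plays the gun animation and sound, then line-traces forward using the Ammo socket and applies damage on a hit.
; Guard enemies get a spawned blood decal actor, while other hits get a temporary attached bullet-hole decal.
; The laser function toggles LmgLaser visibility with debug prints, and Reload only calls the parent.
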(fn `LaserPointerXD`
  (bind _lmglaser (`self.LmgLaser`))
  (`parent.LaserPointerXD`)
  (if (`self.laser visible`)
    (`SceneComponent.SetVisibility` _lmglaser false false)
    (`KismetSystemLibrary.PrintString` "Toggle off")
    (set `self.laser visible` false)
    (else
      (`SceneComponent.SetVisibility` _lmglaser true false)
      (`KismetSystemLibrary.PrintString` "Toggle on")
      (set `self.laser visible` true))))

(fn `Reload`
  (`parent.Reload`))

(fn `Shoot`
  (bind _weaponskeletalmesh (`self.WeaponSkeletalmesh`))
  (bind (_returnvalue_location _returnvalue_rotation) (`KismetMathLibrary.BreakTransform` (`SceneComponent.GetSocketTransform` _weaponskeletalmesh "Ammo" "RTS_World")))
  (`parent.Shoot`)
  (`SkeletalMeshComponent.PlayAnimation` _weaponskeletalmesh "/Game/WeaponsAndAmmo/SM_MachineGun_01_Skel_Sequence.SM_MachineGun_01_Skel_Sequence" false)
  (`GameplayStatics.PlaySoundAtLocation` "/Game/FirstPerson/Blueprints/GunSounds/Pistol.Pistol" _returnvalue_location (struct) 1.0 1.0 0.0 null null null null)
  (bind (_outhit _returnvalue) (`KismetSystemLibrary.LineTraceSingle` :`Start` _returnvalue_location :`End` (+ (`SceneComponent.K2_GetComponentLocation` _weaponskeletalmesh) (* (`KismetMathLibrary.GetForwardVector` _returnvalue_rotation) 15000.0)) :`TraceChannel` "TraceTypeQuery3" :`DrawDebugType` "ForOneFrame" :`TraceColor` (struct :`R` 0.508158 :`G` 1.0 :`B` 0.468852 :`A` 1.0)))
  (if _returnvalue
    (bind (_bblockinghit _binitialoverlap _time _distance _location _impactpoint _normal _impactnormal _physmat _hitactor _hitcomponent) (`GameplayStatics.BreakHitResult` _outhit))
    (`GameplayStatics.ApplyDamage` _hitactor 15.0)
    (cast `/Game/Enemies/AI/BP_Enemy_Base_Guard` _hitactor
      (:`then`
        ;[0.487 0.001268 0.004079] Bloodsplatter
        (`|SpawnActorFromClass` "/Game/Megascans/Decals/blooddecal.blooddecal_C" (`KismetMathLibrary.MakeTransform` _location (`KismetMathLibrary.Conv_VectorToRotator` _impactnormal)) "Undefined" "MultiplyWithRoot" null null))
      (:`CastFailed`
        ;[0.3333 0.3333 0.3333] BULLET HOLE decal when hit looks wierd on ground what can i do :-D
        (`GameplayStatics.SpawnDecalAttached` "/Game/WeaponsAndAmmo/BulletHoleMaterial.BulletHoleMaterial" (10.0 10.0 10.0) _hitcomponent "None" _location (struct) "KeepWorldPosition" 10.0)))))

(fn `UserConstructionScript`
  (`parent.UserConstructionScript`))