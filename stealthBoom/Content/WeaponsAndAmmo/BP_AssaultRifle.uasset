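; Assault rifle child Blueprint, used by the player and enemy guards, that extends its parent's shooting and laser pointer and mounts an iron-sights camera on the mesh.
; Shoot plays a sound and line-traces from the Ammo socket to apply damage, with bonus damage for guard headshots.
; Hits spawn blood or bullet-hole decals through separate guard and player cast checks.
; LaserPointerXD stretches the laser to its trace distance while LaserVisible is false.
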(event `self.ReceiveBeginPlay`
  (`parent.ReceiveBeginPlay`))

(fn `AddAmmo`
  (params (AmmoAmount :type Integer))
  (`parent.AddAmmo` 0))

(fn `BaseWeaponMelee`
  (`parent.BaseWeaponMelee`))

(fn `LaserPointerXD`
  (bind _weaponskeletalmesh (`self.WeaponSkeletalmesh`))
  (bind (_returnvalue_location _returnvalue_rotation) (`KismetMathLibrary.BreakTransform` (`SceneComponent.GetSocketTransform` _weaponskeletalmesh "Ammo" "RTS_World")))
  (`parent.LaserPointerXD`)
  (if (not (`self.laser visible`))
    (bind _asbp_first_person_character (cast `/Game/FirstPerson/Blueprints/BP_FirstPersonCharacter` (`GameplayStatics.GetPlayerCharacter` 0)))
    (set `self.PlayerRefInsideAK` _asbp_first_person_character)
    (bind (_outhit _returnvalue) (`KismetSystemLibrary.LineTraceSingle` :`Start` _returnvalue_location :`End` (+ (`SceneComponent.K2_GetComponentLocation` _weaponskeletalmesh) (* (`KismetMathLibrary.GetForwardVector` _returnvalue_rotation) (`self.MaxLaserRange`))) :`TraceChannel` "TraceTypeQuery2" :`TraceColor` (struct :`R` 0.48515 :`B` 0.456411 :`A` 1.0)))
    (if _returnvalue
      (`SceneComponent.SetRelativeScale3D` (`self.RealLaser`) (`KismetMathLibrary.MakeVector` (`.Distance` (`GameplayStatics.BreakHitResult` _outhit)) 0.5 0.5))
      (else
        (`SceneComponent.SetRelativeScale3D` (`self.RealLaser`) (`KismetMathLibrary.MakeVector` (`self.MaxLaserRange`) 0.5 0.5))))))

(fn `Reload`
  (`parent.Reload`))

(fn `Shoot`
  (bind _weaponskeletalmesh (`self.WeaponSkeletalmesh`))
  (bind (_returnvalue_location _returnvalue_rotation) (`KismetMathLibrary.BreakTransform` (`SceneComponent.GetSocketTransform` _weaponskeletalmesh "Ammo" "RTS_World")))
  (`parent.Shoot`)
  (`GameplayStatics.PlaySoundAtLocation` "/Game/FirstPerson/Blueprints/GunSounds/AK.AK" _returnvalue_location (struct) 1.0 1.0 0.0 null null null null)
  (bind (_outhit _returnvalue) (`KismetSystemLibrary.LineTraceSingle` :`Start` _returnvalue_location :`End` (+ (`SceneComponent.K2_GetComponentLocation` _weaponskeletalmesh) (* (`KismetMathLibrary.GetForwardVector` _returnvalue_rotation) 15000.0)) :`TraceChannel` "TraceTypeQuery3" :`DrawDebugType` "ForOneFrame" :`TraceColor` (struct :`R` 1.0 :`G` 0.917778 :`B` 0.134194 :`A` 1.0)))
  (if _returnvalue
    (bind (_bblockinghit _binitialoverlap _time _distance _location _impactpoint _normal _impactnormal _physmat _hitactor _hitcomponent) (`GameplayStatics.BreakHitResult` _outhit))
    (`GameplayStatics.ApplyDamage` _hitactor 20.0)
    ;[1 1 1] First check if enemy cause more likely that player starts shooting first and added player here cause all enemies have this weapon :-D
    (`|ExecutionSequence`
      (:`then_0`
        (bind _asbp_enemy_base_guard (cast `/Game/Enemies/AI/BP_Enemy_Base_Guard` _hitactor)
          (:`then`
            (if (== _hitcomponent (`/Game/Enemies/AI/BP_Enemy_Base.HeadHitBox` _asbp_enemy_base_guard))
              (`GameplayStatics.ApplyDamage` _hitactor 80.0)
              ;[0.487 0.001268 0.004079] Bloodsplatter
              (`|SpawnActorFromClass` "/Game/Megascans/Decals/blooddecal.blooddecal_C" (`KismetMathLibrary.MakeTransform` _location (`KismetMathLibrary.Conv_VectorToRotator` _impactnormal)) "Undefined" "MultiplyWithRoot" null null :!label _label)))
          (:`CastFailed`
            ;[0.3333 0.3333 0.3333] BULLET HOLE decal when hit looks wierd on ground what can i do :-D
            (`GameplayStatics.SpawnDecalAttached` "/Game/WeaponsAndAmmo/BulletHoleMaterial.BulletHoleMaterial" (10.0 10.0 10.0) _hitcomponent "None" _location (struct) "KeepWorldPosition" 10.0 :!label _label_2))))
      (:`then_1`
        (cast `/Game/FirstPerson/Blueprints/BP_FirstPersonCharacter` _hitactor
          (:`then`
            (goto _label))
          (:`CastFailed`
            (goto _label_2)))))))

(fn `UserConstructionScript`
  (`parent.UserConstructionScript`)
  (`SceneComponent.K2_AttachToComponent` (`self.IronSightsCamera`) (`self.WeaponSkeletalmesh`) "IronSight" "KeepRelative" "KeepRelative" "KeepRelative" true))