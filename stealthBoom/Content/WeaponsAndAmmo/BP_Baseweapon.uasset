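; Base weapon Blueprint with a working melee attack and empty Shoot, Reload and LaserPointerXD functions.
; On BeginPlay, if the player is BP_FirstPersonCharacter, IsEquiped either applies the overlay material or deactivates Weaponspin and clears the overlay.
; BaseWeaponMelee line-traces from the Ammo socket along its forward direction with persistent debug drawing, damages the hit actor and spawns a blood decal on BP_Enemy hits.
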(event `self.ReceiveBeginPlay`
  (cast `/Game/FirstPerson/Blueprints/BP_FirstPersonCharacter` (`GameplayStatics.GetPlayerCharacter` 0))
  (if (`self.IsEquiped`)
    (`MeshComponent.SetOverlayMaterial` (`self.WeaponSkeletalmesh`) "/Game/WeaponsAndAmmo/WeaponOverlay.WeaponOverlay")
    (else
      (`ActorComponent.SetActive` (`self.weaponspin`) false false)
      (`MeshComponent.SetOverlayMaterial` (`self.WeaponSkeletalmesh`) null))))

(fn `BaseWeaponMelee`
  (bind _weaponskeletalmesh (`self.WeaponSkeletalmesh`))
  (bind (_returnvalue_location _returnvalue_rotation) (`KismetMathLibrary.BreakTransform` (`SceneComponent.GetSocketTransform` _weaponskeletalmesh "Ammo" "RTS_World")))
  (bind (_outhit _returnvalue) (`KismetSystemLibrary.LineTraceSingle` :`Start` _returnvalue_location :`End` (+ (`SceneComponent.K2_GetComponentLocation` _weaponskeletalmesh) (* (`KismetMathLibrary.GetForwardVector` _returnvalue_rotation) 240.0)) :`TraceChannel` "TraceTypeQuery3" :`DrawDebugType` "Persistent" :`TraceHitColor` (struct :`R` 0.998785 :`G` 0.279046 :`B` 1.0 :`A` 1.0)))
  (if _returnvalue
    (bind (_bblockinghit _binitialoverlap _time _distance _location _impactpoint _normal _impactnormal _physmat _hitactor) (`GameplayStatics.BreakHitResult` _outhit))
    (`GameplayStatics.ApplyDamage` _hitactor 100.0)
    (cast `/Game/Enemies/BP_Enemy` _hitactor)
    (`|SpawnActorFromClass` "/Game/Megascans/Decals/blooddecal.blooddecal_C" (`KismetMathLibrary.MakeTransform` _location (`KismetMathLibrary.Conv_VectorToRotator` _impactnormal)) "Undefined" "MultiplyWithRoot" null null)))

(fn `LaserPointerXD`)

(fn `Reload`)

(fn `Shoot`)

(fn `UserConstructionScript`)