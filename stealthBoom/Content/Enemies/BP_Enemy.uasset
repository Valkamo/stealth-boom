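; Enemy Blueprint that drives chase and patrol through its AI blackboard and handles its own health and death.
; PawnSensing sightings or the follow event set HasSeenPlayer, and Tick clears it once the player is far enough away horizontally.
; Damage lowers Heltti, reporting a player-instigated damage event to AI perception while alive.
; At zero health the mesh ragdolls, then the actor is destroyed after a short delay.
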(event `follow`
  ;[0.8286 1 0.717] chase  mode activeting
  (set `self.seeing?` true :!label _label)
  (`BlackboardComponent.SetValueAsBool` (`AIBlueprintHelperLibrary.GetBlackboard` (`AIBlueprintHelperLibrary.GetAIController` self)) "HasSeenPlayer" true))

(event `self.PawnSensing.OnSeePawn`
  (params (Pawn :type "Pawn Object Reference"))
  ;[0.8286 1 0.717] chase  mode activeting
  (goto _label))

(event `self.ReceiveTick`
  (params (DeltaSeconds :type "Float (single-precision)"))
  ;[1 0.8214 0.7195] back to patrolling
  (if (>= (`self.GetHorizontalDistanceTo` (`GameplayStatics.GetPlayerCharacter` 0)) 1000.0)
    ;[0.8286 1 0.717] chase  mode activeting
    (`BlackboardComponent.SetValueAsBool` (`AIBlueprintHelperLibrary.GetBlackboard` (`AIBlueprintHelperLibrary.GetAIController` self)) "HasSeenPlayer" false)))

(event `self.ReceiveAnyDamage`
  (params (Damage :type "Float (single-precision)") (DamageType :type "DamageType Object Reference") (InstigatedBy :type "Controller Object Reference") (DamageCauser :type "Actor Object Reference"))
  (bind _returnvalue (`GameplayStatics.GetPlayerCharacter` 0))
  (bind _mesh (`self.Mesh`))
  (bind _heltti (`self.heltti`))
  ;[1 1 1] Applying damage and setting up ragdoll :-D
  (if (> _heltti 0.0)
    (set `self.heltti` (- _heltti Damage))
    (`KismetSystemLibrary.PrintString` (`KismetStringLibrary.Conv_DoubleToString` _heltti) true true (struct :`R` 0.25791 :`G` 1.0 :`A` 1.0))
    (if (<= _heltti 0.0)
      (`PrimitiveComponent.SetSimulatePhysics` _mesh true)
      (`SkeletalMeshComponent.SetPhysicsBlendWeight` _mesh 1.0)
      (`PrimitiveComponent.SetCollisionEnabled` _mesh "QueryAndPhysics")
      (`KismetSystemLibrary.Delay` 1.7)
      (`self.K2_DestroyActor`)
      (else
        (`KismetSystemLibrary.PrintString` "alive")
        (`AISense_Damage.ReportDamageEvent` self _returnvalue 10.0 (`self.K2_GetActorLocation` _returnvalue))))))

(fn `UserConstructionScript`)