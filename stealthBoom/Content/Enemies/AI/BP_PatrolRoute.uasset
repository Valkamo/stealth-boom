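; BP_PatrolRoute is a spline-based patrol path that supplies waypoints for enemy AI.
; IncrementPatrolRoute steps PatrolIndex along the spline points by Direction, flipping Direction at the last and first points so the route ping-pongs instead of looping.
; GetSplinePointAsWorldPosition returns the current point's location in world space rather than relative to the actor.
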(event `IncrementPatrolRoute`
  ;[1 1 1] Increment current point
  (bind _output_get (set `self.PatrolIndex` (+ (`self.PatrolIndex`) (`self.Direction`))))
  (if (== _output_get (- (`SplineComponent.GetNumberOfSplinePoints` (`self.PatrolRoute`)) 1))
    (set `self.Direction` -1)
    (elif (== (`self.PatrolIndex`) 0)
      (set `self.Direction` 1))))

(fn `GetSplinePointAsWorldPosition`
  (returns (loctaion :type "Vector Structure"))
  ;[1 1 1] make sure coordinate space is set to World not local so we don't get relative location to actor
  (return (`SplineComponent.GetLocationAtSplinePoint` (`self.PatrolRoute`) (`self.PatrolIndex`) "World")))

(fn `UserConstructionScript`)