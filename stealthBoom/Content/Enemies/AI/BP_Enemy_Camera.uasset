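; Security camera enemy that raises a local alarm when its AI controller signals an attack.
; It binds to the controller's attack and peace events, switching its point and spot lights between red and blue.
; On attack it closes doors within LocalRange and sets guards in that range to attack the player.
; It then plays a cooldown-limited shutter sound at the player's location and calls OnAttackEnd.
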(event `SetPassiveLight`
  ;[1 1 1] for patrolling
  (`LightComponent.SetLightColor` (`self.PointLight`) (struct :`G` 0.097587 :`B` 0.597202 :`A` 1.0) true)
  (`LightComponent.SetLightColor` (`self.SpotLight`) (struct :`G` 0.097587 :`B` 0.597202 :`A` 1.0) true))

(event `self.ReceiveBeginPlay`
  (bind _asaic_enemy_camera (cast `/Game/Enemies/AI/AIC_Enemy_Camera` (`self.GetController`)))
  (add `/Game/Enemies/AI/AIC_Enemy_Camera.AttackTime` _asaic_enemy_camera (delegate `/Game/Enemies/AI/BPI_EnemyAI.Attack`))
  (add `/Game/Enemies/AI/AIC_Enemy_Camera.PeaceTime` _asaic_enemy_camera (delegate `SetPassiveLight`)))

(event `/Game/Enemies/AI/BPI_EnemyAI.Attack`
  (`self.SetLightToAttacking`)
  (bind _outactors (`GameplayStatics.GetAllActorsOfClass` "/Game/Door/Door.Door_C"))
  (for _array_element _outactors
    (`self.LockTheDoor` _array_element _array_element))
  (`self.CallAllLocalGaurds`)
  (`|ExecutionSequence`
    (:`then_0`
      (`/Engine/EditorBlueprintResources/StandardMacros.DoOnce` false :!label _label
        (:`Completed`
          (`self.PlayAttackSound`)
          (`KismetSystemLibrary.Delay` 5.0)
          (goto _label :!via `Reset`))))
    (:`then_1`
      (`self.OnAttackEnd`))))

(event `SetLightToAttacking`
  (`LightComponent.SetLightColor` (`self.PointLight`) (struct :`R` 0.78125 :`A` 1.0) true)
  (`LightComponent.SetLightColor` (`self.SpotLight`) (struct :`R` 0.78125 :`A` 1.0) true))

(fn `CallAllLocalGaurds`
  (bind _returnvalue (`GameplayStatics.GetPlayerCharacter` 0))
  (bind _outactors (`GameplayStatics.GetAllActorsOfClass` "/Game/Enemies/AI/BP_Enemy_Base_Guard.BP_Enemy_Base_Guard_C"))
  (for _array_element _outactors
    (if (<= (`self.GetDistanceTo` _array_element self) (`self.LocalRange`))
      (bind _asaic_enemy_base (cast `/Game/Enemies/AI/AIC_Enemy_base` (`AIBlueprintHelperLibrary.GetAIController` _array_element)))
      (`/Game/Enemies/AI/AIC_Enemy_base.Set State As Attacking` _asaic_enemy_base _returnvalue (`self.K2_GetActorLocation` _returnvalue)))))

(fn `LockTheDoor`
  (params (self2 :type "/Game/Door/Door Object Reference") (self3 :type "Actor Object Reference"))
  (if (<= (`self.GetDistanceTo` self3 self) (`self.LocalRange`))
    (`/Game/Door/Door.CloseTheDoor` self2)))

(fn `PlayAttackSound`
  (`GameplayStatics.PlaySoundAtLocation` "/Engine/VREditor/Sounds/UI/Camera_Shutter.Camera_Shutter" (`self.K2_GetActorLocation` (`GameplayStatics.GetPlayerCharacter` 0)) (struct) 3.0 1.0 0.0 null null null null))

(fn `UserConstructionScript`
  (`parent.UserConstructionScript`))