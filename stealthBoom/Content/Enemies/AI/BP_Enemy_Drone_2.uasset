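; Drone enemy that works as a spotter, raising the alarm on the player.
; Attack puts the AI controller of every BP_Enemy_Base_Guard into the attacking state against the player, plays a camera shutter sound at the player and signals attack end.
; Its point light turns red once guards are alerted and blue when set passive for patrolling.
; GetIdealRange supplies fixed attack and defend radii.
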(event `SetPassiveLight`
  ;[1 1 1] for patrolling
  (`LightComponent.SetLightColor` (`self.PointLight`) (struct :`G` 0.097587 :`B` 0.597202 :`A` 1.0) true))

(event `/Game/Enemies/AI/BPI_EnemyAI.Attack`
  ;[1 1 1] for attacking
  (bind _outactors (`GameplayStatics.GetAllActorsOfClass` "/Game/Enemies/AI/BP_Enemy_Base_Guard.BP_Enemy_Base_Guard_C"))
  (for _array_element _outactors
    (`KismetSystemLibrary.PrintString` (`KismetSystemLibrary.GetDisplayName` _array_element))
    (bind _asaic_enemy_base (cast `/Game/Enemies/AI/AIC_Enemy_base` (`AIBlueprintHelperLibrary.GetAIController` _array_element)))
    (`/Game/Enemies/AI/AIC_Enemy_base.SetStateAsAttacking` _asaic_enemy_base (`GameplayStatics.GetPlayerCharacter` 0))
    (`GameplayStatics.PlaySoundAtLocation` "/Engine/VREditor/Sounds/UI/Camera_Shutter.Camera_Shutter" (`self.K2_GetActorLocation` (`GameplayStatics.GetPlayerCharacter` 0)) (struct) 1.0 1.0 0.0 null null null null :!label _label)
    (`self.OnAttackEnd`))
  (`LightComponent.SetLightColor` (`self.PointLight`) (struct :`R` 0.78125 :`A` 1.0) true)
  (goto _label))

(fn `GetIdealRange`
  (returns (AttackRaduis :type "Float (double-precision)") (DefendRadius :type "Float (double-precision)"))
  (return 350.0 450.0))

(fn `UserConstructionScript`
  (`parent.UserConstructionScript`))