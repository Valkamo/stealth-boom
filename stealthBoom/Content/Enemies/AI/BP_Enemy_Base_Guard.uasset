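; Guard enemy that spawns armed with an assault rifle and targets the player.
; On BeginPlay it sets the player as its AI controller's attack target, then attaches a spawned rifle to its right hand, disabling the weapon's spin and clearing its overlay material.
; Attack fires the rifle and immediately signals attack end.
; It also supplies fixed attack and defend ranges and exposes its patrol route.
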(event `self.ReceiveBeginPlay`
  (bind _weaponactor (`self.WeaponActor`))
  ;[1 1 1] Set Player as Attack Target for Guard
  (bind _asaic_enemy_base (cast `/Game/Enemies/AI/AIC_Enemy_base` (`self.GetController`)))
  (bind _output_get (set `/Game/Enemies/AI/AIC_Enemy_base.Attack Target` (`GameplayStatics.GetPlayerCharacter` 0) _asaic_enemy_base))
  (`/Game/Enemies/AI/AIC_Enemy_base.SetAttackTarget` _asaic_enemy_base _output_get)
  (bind _returnvalue (`|SpawnActorFromClass` "/Game/WeaponsAndAmmo/BP_AssaultRifle.BP_AssaultRifle_C" (`KismetMathLibrary.MakeTransform` (0.0 0.0 0.0)) "Undefined" "MultiplyWithRoot" null null))
  (set `self.WeaponActor` _returnvalue)
  (set `/Game/WeaponsAndAmmo/BP_Baseweapon.IsTaken` true _returnvalue)
  (`self.K2_AttachToComponent` _returnvalue (`self.Mesh`) "RightHandSocket" "SnapToTarget" "SnapToTarget" "KeepRelative" true)
  (set `self.IsWieldingWeapon` true)
  (`ActorComponent.SetActive` (`/Game/WeaponsAndAmmo/BP_Baseweapon.weaponspin` _weaponactor) false false)
  (`MeshComponent.SetOverlayMaterial` (`/Game/WeaponsAndAmmo/BP_Baseweapon.WeaponSkeletalmesh` _weaponactor) null))

(event `/Game/Enemies/AI/BPI_EnemyAI.Attack`
  (if (`self.IsWieldingWeapon`)
    (`/Game/WeaponsAndAmmo/BP_Baseweapon.Shoot` (`self.WeaponActor`))
    (`self.OnAttackEnd`)))

(fn `GetIdealRange`
  (returns (AttackRaduis :type "Float (double-precision)") (DefendRadius :type "Float (double-precision)"))
  (return 200.0 600.0))

(fn `GetPatrolRoute`
  (returns (PatrolRoute :type "/Game/Enemies/AI/BP_PatrolRoute Object Reference"))
  (return (`self.PatrolRoute`)))

(fn `UserConstructionScript`
  (`parent.UserConstructionScript`))