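; BP_Enemy_Guard is an enemy guard character that wields an assault rifle.
; On BeginPlay it spawns a BP_AssaultRifle, attaches it to the mesh's right-hand socket, flags itself as wielding and fires the weapon-equipped notification.
; Attack plays a rifle-firing montage and signals attack end whether the montage completes or is interrupted.
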(event `self.ReceiveBeginPlay`
  (`self.EquipWeapon`))

(event `/Game/Enemies/AI/BPI_EnemyAI.EquipWeapon`
  (bind _returnvalue (`|SpawnActorFromClass` "/Game/WeaponsAndAmmo/BP_AssaultRifle.BP_AssaultRifle_C" (`KismetMathLibrary.MakeTransform` (0.0 0.0 0.0)) "Undefined" "MultiplyWithRoot" null null))
  (bind _output_get (set `self.WeaponActor` _returnvalue))
  (`self.K2_AttachToComponent` _output_get (`self.Mesh`) "RightHandSocket" "KeepRelative" "KeepRelative" "KeepRelative" true)
  (set `self.IsWieldingWeapon` true)
  (`self.OnWeaponEquipped`))

(event `/Game/Enemies/AI/BPI_EnemyAI.Attack`
  (`|PlayMontage` (`self.Mesh`) "/Game/Animationpack/Basic_Shooter_Pack/firing_rifle_Montage.firing_rifle_Montage"
    (:`OnCompleted`
      _)
    (:`OnInterrupted`
      _))
  (`self.OnAttackEnd`))

(fn `UserConstructionScript`
  (`parent.UserConstructionScript`))