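; Base enemy character Blueprint that handles health, death and data getters for ideal range, patrol route and movement speed.
; Non-lethal damage reports a damage sense event blamed on player 0; lethal damage ragdolls the mesh, then destroys weapon and actor after a delay.
; SetMovementSpeed maps a movement state to walk speed.
; Equip and unequip events are empty, with rifle spawn and montage logic left disconnected.
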(event `/Game/Enemies/AI/BPI_EnemyAI.EquipWeapon`
  ;[1 1 1] will call the gun bp here
)

(event `/Game/Enemies/AI/BPI_EnemyAI.UnEquipWeapon`
  ;[1 1 1] will call the gun bp here
)

(event `self.ReceiveAnyDamage`
  (params (Damage :type "Float (single-precision)") (DamageType :type "DamageType Object Reference") (InstigatedBy :type "Controller Object Reference") (DamageCauser :type "Actor Object Reference"))
  (bind _returnvalue (`GameplayStatics.GetPlayerCharacter` 0))
  (bind _mesh (`self.Mesh`))
  (bind _heltti (`self.heltti`))
  ;[1 1 1] Applying damage and setting up ragdoll :-D
  (if (> _heltti 0.0)
    (set `self.heltti` (- _heltti Damage))
    (if (<= _heltti 0.0)
      (`PrimitiveComponent.SetSimulatePhysics` _mesh true)
      (`SkeletalMeshComponent.SetPhysicsBlendWeight` _mesh 1.0)
      (`PrimitiveComponent.SetCollisionEnabled` _mesh "QueryAndPhysics")
      (`KismetSystemLibrary.Delay` 1.7)
      (bind _weaponactor (`self.WeaponActor`)
        (:`then`
          (`self.K2_DestroyActor` _weaponactor))
        (:`else`
          _))
      (`self.K2_DestroyActor`)
      (else
        (`AISense_Damage.ReportDamageEvent` self _returnvalue 10.0 (`self.K2_GetActorLocation` _returnvalue))))))

(fn `GetIdealRange`
  (returns (AttackRaduis :type "Float (double-precision)") (DefendRadius :type "Float (double-precision)"))
  (return 150.0 350.0))

(fn `GetPatrolRoute`
  (returns (PatrolRoute :type "/Game/Enemies/AI/BP_PatrolRoute Object Reference"))
  (return (`self.PatrolRoute`)))

(fn `SetMovementSpeed`
  (params (Speed :type "/Game/Enemies/AI/Enums/E_Movement_Speed Enum" :default "NewEnumerator0"))
  (returns (SpeedValue :type "Float (double-precision)"))
  (bind _output_get (set `CharacterMovementComponent.MaxWalkSpeed` (select `/Game/Enemies/AI/Enums/E_Movement_Speed` Speed :`NewEnumerator1` 100.0 :`NewEnumerator2` 300.0 :`NewEnumerator3` 500.0 :!type "Float (single-precision)") (`self.CharacterMovement`)))
  (return _output_get))

(fn `UserConstructionScript`)