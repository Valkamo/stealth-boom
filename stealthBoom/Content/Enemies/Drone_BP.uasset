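; Enemy drone Blueprint that reports whether it has seen the player to its AI controller's Blackboard.
; PawnSensing sets the HasSeenPlayer key when it sees a pawn, with no check that the pawn is the player.
; Tick clears the key whenever the first player's character is at or beyond a fixed horizontal distance, ignoring height.
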(event `self.PawnSensing.OnSeePawn`
  (params (Pawn :type "Pawn Object Reference"))
  (`BlackboardComponent.SetValueAsBool` (`AIBlueprintHelperLibrary.GetBlackboard` (`AIBlueprintHelperLibrary.GetAIController` self)) "HasSeenPlayer" true))

(event `self.ReceiveTick`
  (params (DeltaSeconds :type "Float (single-precision)"))
  (if (>= (`self.GetHorizontalDistanceTo` (`GameplayStatics.GetPlayerCharacter` 0)) 1000.0)
    (`BlackboardComponent.SetValueAsBool` (`AIBlueprintHelperLibrary.GetBlackboard` (`AIBlueprintHelperLibrary.GetAIController` self)) "HasSeenPlayer" false)))

(fn `UserConstructionScript`)